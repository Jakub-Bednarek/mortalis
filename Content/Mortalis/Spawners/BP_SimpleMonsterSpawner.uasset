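; BP_SimpleMonsterSpawner is a sample monster spawner that releases slime enemies in timed waves around itself.
; On BeginPlay it configures its ActorSpawner with a periodic interval, a wave limit, a per-spawn count, a radius and a pool holding only BP_SlimeEnemy.
; It also enables NavMesh position selection on the spawner and leaves all spawning logic to it, with no Tick, overlap or construction logic of its own.
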(event EventBeginPlay
  ;[0.73 1 0.5398] Sample Spawner Configuration
  (Class|ActorSpawnerComponent|EnablePeriodicSpawn (Variables|Default|GetActorSpawner) 4.0 10)
  (Class|ActorSpawnerComponent|SetActorSpawnCount (Variables|Default|GetActorSpawner) 3)
  (Class|ActorSpawnerComponent|SetSpawnRadius (Variables|Default|GetActorSpawner) 3e+03)
  (Class|ActorSpawnerComponent|SetActorSpawnPool (Variables|Default|GetActorSpawner) (Utilities|Array|MakeArray "/Game/Mortalis/Enemies/BP_SlimeEnemy.BP_SlimeEnemy_C"))
  (Class|ActorSpawnerComponent|EnableNavMeshPositionSelection (Variables|Default|GetActorSpawner)))

(event Collision|EventActorBeginOverlap
  (params (OtherActor :type Actor%20Object%20Reference)))

(event EventTick
  (params (DeltaSeconds :type Float%20%28single-precision%29)))

(fn ConstructionScript)