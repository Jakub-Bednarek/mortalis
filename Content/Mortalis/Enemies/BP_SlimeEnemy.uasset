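; Slime enemy that chases the player, deals contact damage and can be killed by projectiles.
; A FollowPlayer component starts following on BeginPlay, and actor overlaps are sorted by tag.
; Projectiles feed their damage into the EnemyHealth component and are notified of the hit, while player contact calls the archer's hit handler with fixed damage.
; At zero health it fires a death event passing Experience, disables mesh collision and destroys itself.
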(event OnDamageTaken(EnemyHealth))

(event OnZeroHealth(EnemyHealth)
  (Default|CallOnDeathEvent (Variables|Default|GetExperience))
  (Collision|SetCollisionEnabled (Variables|Default|GetSkeletalMesh) "NoCollision")
  (Actor|DestroyActor))

(event EventBeginPlay
  (Class|FollowPlayerComponent|SetFollowingEnabled (Variables|Default|GetFollowPlayer) true))

(event Collision|EventActorBeginOverlap
  (params (OtherActor :type Actor%20Object%20Reference))
  (if (Actor|ActorHasTag OtherActor "Projectile")
    (bind _asbasic_projectile (Utilities|Casting|CastToBasicProjectile OtherActor))
    (Class|EnemyHealthComponent|TakeDamage (Variables|Default|GetEnemyHealth) (Class|BasicProjectile|GetDamage _asbasic_projectile))
    (Class|BasicProjectile|OnCollisionEnter _asbasic_projectile "Enemy")
    (elif (Actor|ActorHasTag OtherActor "Player")
      (bind _asarcher_character (Utilities|Casting|CastToArcherCharacter OtherActor)
        (:then
          (Default|CallOnEnemyHit _asarcher_character 15.0))
        (:CastFailed
          (Development|PrintString "Cast failed"))))))

(fn ConstructionScript)